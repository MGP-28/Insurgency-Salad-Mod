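; Mutator that resupplies a spawned soldier when input key 0 is held over 3.5 seconds while the soldier stands at its spawn location.
; After a short spawn delay it records the location, then polls through a tiny-delay loop until both conditions hold, ending after one resupply.
; The key is read from player controller 0, and the position must match exactly.
; GetRequiredAssets builds its set from AdditionalAssets.
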(event `self.OnPlayerSpawned`
  (params (Soldier :type "INSSoldier Object Reference") (NewPlayer :type "Controller Object Reference") (StartRotation :type "Rotator Structure (by ref)"))
  (bind _returnvalue (`GameplayStatics.GetPlayerController` 0))
  (bind _returnvalue_2 (`Actor.K2_GetActorLocation` Soldier))
  (`KismetSystemLibrary.Delay` 0.2)
  (set `self.PlayerStartingLocation` _returnvalue_2)
  (`/Engine/EditorBlueprintResources/StandardMacros.Gate` false :!label _label
    (:`Exit`
      (if (> (`PlayerController.GetInputKeyTimeDown` _returnvalue "Zero") 3.5)
        (if (`KismetMathLibrary.EqualExactly_VectorVector` (`self.PlayerStartingLocation`) _returnvalue_2) :!label _label_2
          _
          (else
            (`KismetSystemLibrary.Delay` 1e-06 :!label _label_3)
            (goto _label)))
        (elif (> (`PlayerController.GetInputKeyTimeDown` _returnvalue "Zero") 3.5)
          (goto _label_2)
          (else
            (goto _label_3))))
      (`INSSoldier.PerformResupply` Soldier))))

(fn `GetRequiredAssets`
  (returns (OutAssetPaths :type "Set of SoftObjectPath Structure"))
  (bind _set (`|MakeSet`))
  (for _array_element (`self.AdditionalAssets`)
    (`BlueprintSetLibrary.Set_Add` _set _array_element))
  (return _set))