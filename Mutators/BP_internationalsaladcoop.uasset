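; Co-op mutator that strips DShK and M2HB shielded mounted weapons and flare pallets shortly after each round starts or ends.
; A post-load check compares TryGuessingAsshole to a hardcoded number, printing it and setting IsPurge on mismatch, apparently as tamper protection.
; Purge destroys every INSSoldier, re-calling itself per soldier.
; That mismatch and many player, team, faction and objective events call Purge directly, bypassing the IsPurge-gated wrapper.
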(event `self.OnRoundStarted`
  (`KismetSystemLibrary.Delay` 1.0)
  (bind _outactors (`GameplayStatics.GetAllActorsOfClass` "/OldDogs/Items/Firesupport/INS/BP_MountedWeapon_DShK_Shield_OD.BP_MountedWeapon_DShK_Shield_OD_C" :!label _label))
  (`Actor.K2_DestroyActor` _outactors)
  (bind _outactors_2 (`GameplayStatics.GetAllActorsOfClass` "/OldDogs/Items/Firesupport/SEC/BP_MountedWeapon_M2HB_Shield_OD.BP_MountedWeapon_M2HB_Shield_OD_C"))
  (`Actor.K2_DestroyActor` _outactors_2)
  (bind _outactors_3 (`GameplayStatics.GetAllActorsOfClass` "/OldDogs/Items/Utility/Flare/OD_Flare_Pallet.OD_Flare_Pallet_C"))
  (`Actor.K2_DestroyActor` _outactors_3))

(event `self.OnRoundOver`
  (params (RoundEndReason :type "ERoundConclusion Enum" :default "Generic") (WinningTeam :type Byte))
  (`KismetSystemLibrary.Delay` 1.0)
  (goto _label))

(event `self.InitializeMutatorPostLoad`
  (bind _tryguessingasshole (`self.TryGuessingAsshole`))
  (`KismetSystemLibrary.Delay` 0.2)
  (if (not (== _tryguessingasshole -284110061568.0))
    (`KismetSystemLibrary.PrintString` (`KismetStringLibrary.Conv_DoubleToString` _tryguessingasshole) true true (struct :`R` 1.0 :`G` 0.580683 :`A` 1.0) 10.0)
    (`self.Purge`)
    (set `self.IsPurge` true)))

(event `Purge`
  (`KismetSystemLibrary.Delay` 0.1)
  (bind _outactors (`GameplayStatics.GetAllActorsOfClass` "/Script/Insurgency.INSSoldier"))
  (for _array_element _outactors
    (`Actor.K2_DestroyActor` _array_element)
    (`self.Purge`))
  (`KismetSystemLibrary.PrintString` "PURGED" true true (struct :`R` 1.0 :`G` 0.031819 :`A` 1.0) 10.0))

(event `Purge?`
  (if (`self.IsPurge`)
    (`self.Purge`)))

(event `self.OnFactionsInitialized`
  (params (Teams :type "Array of TeamInfo Object Reference (by ref)"))
  (`self.Purge?` :!label _label_2))

(event `self.OnObjectiveChangeOwnership`
  (params (Objective :type "ObjectiveBase Object Reference") (NewOwners :type Byte))
  (goto _label_2))

(event `self.OnPlayerClassChanged`
  (params (Controller :type "Controller Object Reference") (PlayerClass :type "PlayerClass Object Reference"))
  (goto _label_2))

(event `self.OnPlayerKilledAnyDamage`
  (params (Victim :type "INSSoldier Object Reference") (KillingDamage :type "Float (single-precision)") (Killer :type "Controller Object Reference") (Assister :type "Controller Object Reference") (DamageCauser :type "Actor Object Reference"))
  (goto _label_2))

(event `self.OnPlayerLogin`
  (params (PlayerController :type "PlayerController Object Reference") (Portal :type String) (Options :type String))
  (goto _label_2))

(event `self.OnPlayerLogout`
  (params (Controller :type "Controller Object Reference"))
  (goto _label_2))

(event `self.OnPlayerSpawned`
  (params (Soldier :type "INSSoldier Object Reference") (NewPlayer :type "Controller Object Reference") (StartRotation :type "Rotator Structure (by ref)"))
  (goto _label_2))

(event `self.OnTeamInitialized`
  (params (Team :type "TeamInfo Object Reference"))
  (goto _label_2))

(fn `GetRequiredAssets`
  (returns (OutAssetPaths :type "Set of SoftObjectPath Structure"))
  (bind _set (`|MakeSet`))
  (for _array_element (`self.AdditionalAssets`)
    (`BlueprintSetLibrary.Set_Add` _set _array_element))
  (return _set))