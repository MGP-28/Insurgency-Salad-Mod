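; Mutator that offers soldiers a one-time resupply at their spawn point, triggered by jumping.
; Five seconds after a spawn, a 0.3-second Delay loop compares the soldier's location to the saved spawn location and repeats a short on-screen prompt.
; Rising above the spawn height calls PerformResupply, while moving out of the small radius cancels, each confirmed by a client message.
; Jumps are detected by height change alone; the input-key check never runs.
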(event `Event Message Resupply`
  (bind _asinsplayer_controller (cast `INSPlayerController` (stale `self.OnPlayerSpawned` NewPlayer)))
  (`INSBasePlayerController.ClientMessageText` _asinsplayer_controller "RESUPPLIED" "None" 3.0))

(event `Event Message Moved`
  (bind _asinsplayer_controller (cast `INSPlayerController` (stale `self.OnPlayerSpawned` NewPlayer)))
  (`INSBasePlayerController.ClientMessageText` _asinsplayer_controller "You moved, resupply CANCELED" "None" 3.0))

(event `self.OnPlayerSpawned`
  (params (Soldier :type "INSSoldier Object Reference") (NewPlayer :type "Controller Object Reference") (StartRotation :type "Rotator Structure (by ref)"))
  (bind _returnvalue (`Actor.K2_GetActorLocation` Soldier))
  (bind _output_get (set `self.PlayerStartingLocation` _returnvalue))
  (`KismetSystemLibrary.Delay` 5.0)
  (`/Engine/EditorBlueprintResources/StandardMacros.Gate` false :!label _label
    (:`Exit`
      (if (== _output_get _returnvalue :`ErrorTolerance` 75.0)
        (if (>= (.z _output_get) (- (.z _returnvalue) 0.25))
          (`KismetSystemLibrary.Delay` 0.3)
          (bind _asinsplayer_controller (cast `INSPlayerController` NewPlayer))
          (`INSBasePlayerController.ClientMessageText` _asinsplayer_controller "JUMP to resupply; move along to cancel" "None" 0.1)
          (goto _label)
          (else
            (`INSSoldier.PerformResupply` Soldier)
            (`self.Event Message Resupply`)))
        (else
          (`self.Event Message Moved`))))))