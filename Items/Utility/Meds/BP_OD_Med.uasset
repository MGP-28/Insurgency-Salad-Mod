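; Limited-use handheld med item that heals its owner or spawns a meds projectile on a soldier it hits.
; Repeated swings build a decaying counter that Tick polls on the server to trigger self-healing.
; Self-heal samples health to reject overlapping heals, then raises it gradually to 85% of max.
; Colored emitters, sounds and client messages report results; the item drops and destroys itself after three charges.
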(event `self.ReceiveTick`
  (params (DeltaSeconds :type "Float (single-precision)"))
  (bind _medsusescount (`self.MedsUsesCount`))
  (if (`KismetSystemLibrary.IsServer`)
    (if (>= (`self.SwingCounter`) 3.0)
      (`self.CustomEvent_0`)
      (`KismetSystemLibrary.PrintString` "SH Enabled" true true (struct :`R` 0.039934 :`G` 1.0 :`A` 1.0) 5.0)
      (set `self.SwingCounter` 0.0))
    (if (== (`self.MedsUsesCount_0`) _medsusescount)
      _
      (elif (>= _medsusescount 3)
        (`KismetSystemLibrary.PrintString` "Maximum uses reached" true true (struct :`R` 1.0 :`G` 0.628354 :`B` 0.165041 :`A` 1.0))
        (`self.DropItem`)
        (set `self.bCanPickup` false)
        (`self.Event Meds Depleted`)
        (`KismetSystemLibrary.Delay` 20.0)
        (`self.K2_DestroyActor`)
        (else
          (bind _output_get (set `self.MedsUsesCount_0` _medsusescount))
          (`KismetSystemLibrary.PrintString` (`KismetStringLibrary.Conv_IntToString` _output_get) true true (struct :`R` 0.213452 :`G` 0.123204 :`B` 1.0 :`A` 1.0))
          (bind _asinsplayer_controller (cast `INSPlayerController` (`self.Info Message Target`))
            (:`then`
              (if (`KismetSystemLibrary.IsServer`)
                (`INSBasePlayerController.ClientMessageText` _asinsplayer_controller (`KismetTextLibrary.Conv_StringToText` (`KismetStringLibrary.Concat_StrStr` (`KismetStringLibrary.Conv_IntToString` (- (`self.MedsUsesBase_3`) _output_get)) " charge(s) left")) "None" 6.0)))
            (:`CastFailed`
              (`KismetSystemLibrary.PrintString` "NOOOOOOOOOOOOOT"))))))))

(event `self.BlueprintOnHit`
  (params (Hit :type "HitResult Structure (by ref)"))
  (if (`KismetSystemLibrary.IsServer`)
    (bind _asinssoldier (cast `INSSoldier` (`.HitActor` (`GameplayStatics.BreakHitResult` Hit)))
      (:`then`
        (bind _returnvalue (`|SpawnActorFromClass` "/OldDogs/Items/Utility/Meds/BP_Projectile_OD_Meds.BP_Projectile_OD_Meds_C" (`self.GetTransform` _asinssoldier) "AlwaysSpawn" "OverrideRootScale" self null))
        (set `/OldDogs/Items/Utility/Meds/BP_Projectile_OD_Meds.Info Message Target Proj` (`self.Info Message Target`) _returnvalue)
        (`KismetSystemLibrary.PrintString` "Spawned")
        (set `self.SwingCounter` 0.0))
      (:`CastFailed`
        (`KismetSystemLibrary.PrintString` "Not soldier")))))

(event `self.BlueprintOnSwing`
  (bind _swingcounter (`self.SwingCounter`))
  (if (not (> _swingcounter 3.0))
    (set `self.SwingCounter` (+ _swingcounter 1.0))
    (`KismetSystemLibrary.Delay` 5.0)
    (if (not (== _swingcounter 0.0))
      (set `self.SwingCounter` (- _swingcounter 1.0)))))

(event `CustomEvent_0`
  (bind _pawnowner (`self.PawnOwner`))
  (bind _returnvalue (`self.K2_GetActorLocation` _pawnowner))
  (bind _health (`INSCharacter.Health` _pawnowner))
  (bind _returnvalue_2 (< _health (* (`INSCharacter.MaxHealth` _pawnowner) 0.85)))
  (`KismetSystemLibrary.Delay` 0.2)
  (if (`KismetSystemLibrary.IsServer`)
    (if _returnvalue_2
      (bind _output_get (set `self.InitialHP` _health))
      (`KismetSystemLibrary.Delay` 0.2)
      (if (< _output_get _health)
        (`KismetSystemLibrary.PrintString` "Player already being healed" true true (struct :`R` 0.75 :`G` 0.412263 :`A` 1.0))
        (set `self.Location` _returnvalue)
        (`self.Event_ShowLight_Yellow`)
        (else
          (set `self.Location` _returnvalue)
          (`self.Event_ShowLight_Green`)
          (set `self.MedsUsesCount` (+ (`self.MedsUsesCount`) 1))
          (`KismetSystemLibrary.PrintString` "Healing..." true true (struct :`R` 0.049854 :`G` 1.0 :`B` 0.17456 :`A` 1.0))
          (`/Engine/EditorBlueprintResources/StandardMacros.Gate` false :!label _label
            (:`Exit`
              (if (`INSCharacter.bIsDying` _pawnowner)
                (`KismetSystemLibrary.PrintString` "Actor dead" true true (struct :`R` 0.713542 :`G` 0.65067 :`A` 1.0))
                (elif _returnvalue_2
                  (set `INSCharacter.Health` (+ _health 0.25) _pawnowner)
                  (`KismetSystemLibrary.Delay` 0.1)
                  (goto _label)
                  (else
                    (`KismetSystemLibrary.PrintString` "Healing done" true true (struct :`R` 0.658188 :`G` 0.150553 :`B` 0.78125 :`A` 1.0))
                    (`self.Event_HealingDone`))))))))
      (else
        (`KismetSystemLibrary.PrintString` "Player above 85% HP" true true (struct :`R` 0.75 :`G` 0.412263 :`A` 1.0))
        (set `self.Location` _returnvalue)
        (`self.Event_ShowLight_Red`)))))

(event `self.BlueprintOnEquip`
  (bind _returnvalue (`self.GetInstigatorController` (`self.GetOwner`)))
  (set `self.Info Message Target` _returnvalue)
  (if (`KismetSystemLibrary.IsServer`)
    (bind _asinsplayer_controller (cast `INSPlayerController` _returnvalue))
    (`INSBasePlayerController.ClientMessageText` _asinsplayer_controller (`KismetTextLibrary.Conv_StringToText` (`KismetStringLibrary.Concat_StrStr` (`KismetStringLibrary.Conv_IntToString` (- (`self.MedsUsesBase_3`) (`self.MedsUsesCount`))) " charge(s) left")) "None" 6.0)))

(event `Event_ShowLight_Yellow`
  (if (`KismetSystemLibrary.IsServer`)
    (`KismetSystemLibrary.Delay` 0.2)
    (`GameplayStatics.SpawnEmitterAtLocation` "/OldDogs/Items/Utility/Meds/PS_OD_Meds_Working_Yellow.PS_OD_Meds_Working_Yellow" (`self.Location`) (struct) (5.0 5.0 5.0))
    (bind _asinsplayer_controller (cast `INSPlayerController` (`self.Info Message Target`)))
    (`INSBasePlayerController.ClientMessageText` _asinsplayer_controller "You're already being healed" "None" 6.0)))

(event `Event Meds Depleted`
  (if (`KismetSystemLibrary.IsServer`)
    (bind _asinsplayer_controller (cast `INSPlayerController` (`self.Info Message Target`)))
    (`INSBasePlayerController.ClientMessageText` _asinsplayer_controller "Out of charges, dropped item" "None" 6.0)))

(event `Event_ShowLight_Red`
  (if (`KismetSystemLibrary.IsServer`)
    (`KismetSystemLibrary.Delay` 0.2)
    (`GameplayStatics.SpawnEmitterAtLocation` "/OldDogs/Items/Utility/Meds/PS_OD_Meds_Working_Red.PS_OD_Meds_Working_Red" (`self.Location`) (struct) (5.0 5.0 5.0))
    (bind _asinsplayer_controller (cast `INSPlayerController` (`self.Info Message Target`)))
    (`INSBasePlayerController.ClientMessageText` _asinsplayer_controller "You're above 85% HP, can't be healed" "None" 6.0)))

(event `Event_ShowLight_Green`
  (bind _location (`self.Location`))
  (if (`KismetSystemLibrary.IsServer`)
    (`KismetSystemLibrary.Delay` 0.2)
    (`GameplayStatics.SpawnEmitterAtLocation` "/OldDogs/Items/Utility/Meds/PS_OD_Meds_Working_Green.PS_OD_Meds_Working_Green" _location (struct) (5.0 5.0 5.0))
    (`AkGameplayStatics.SpawnAkComponentAtLocation` "/Game/Audio/wwise/Sandstorm/VO/SecArabMale1/GeneralChatter2/Play_SecArabMale1_GeneralChatter2_Strenuous_Physical_Exertion.Play_SecArabMale1_GeneralChatter2_Strenuous_Physical_Exertion" _location (struct) true)
    (bind _asinsplayer_controller (cast `INSPlayerController` (`self.Info Message Target`)))
    (`INSBasePlayerController.ClientMessageText` _asinsplayer_controller "Healing yourself..." "None" 6.0)))

(event `Event_HealingDone`
  (bind _location (`self.Location`))
  (if (`KismetSystemLibrary.IsServer`)
    (`KismetSystemLibrary.Delay` 0.2)
    (`GameplayStatics.SpawnEmitterAtLocation` "/OldDogs/Items/Utility/Meds/PS_OD_Meds_Working_Green.PS_OD_Meds_Working_Green" _location (struct) (5.0 5.0 5.0))
    (`AkGameplayStatics.SpawnAkComponentAtLocation` "/Game/Audio/wwise/Sandstorm/VO/SecArabMale1/Breathing/Play_SecArabMale1_Breathing_Focus_Exhale.Play_SecArabMale1_Breathing_Focus_Exhale" _location (struct) true)
    (bind _asinsplayer_controller (cast `INSPlayerController` (`self.Info Message Target`)))
    (`INSBasePlayerController.ClientMessageText` _asinsplayer_controller "You're healed up and ready" "None" 12.0)))

(fn `UserConstructionScript`)