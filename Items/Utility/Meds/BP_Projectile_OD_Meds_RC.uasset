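; Med item projectile that heals the soldier in SelfHealRef gradually up to 85% of max health.
; On BeginPlay the server rejects targets above that threshold, or already being healed, detected by sampling health across a short delay.
; Otherwise it increments the owning BP_OD_Med's use count and runs a delayed Gate loop adding health until done or dying.
; Light events give non-server instances colored particles and player messages, plus a sound when healing.
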(event `self.ReceiveBeginPlay`
  (`KismetSystemLibrary.Delay` 0.2)
  (if (`KismetSystemLibrary.IsServer`)
    (bind _asinssoldier (cast `INSSoldier` (`self.SelfHealRef`))
      (:`then`
        (bind _health (`INSCharacter.Health` _asinssoldier))
        (bind _returnvalue (< _health (* (`INSCharacter.MaxHealth` _asinssoldier) 0.85)))
        (if _returnvalue
          (bind _output_get (set `self.InitialHP` _health))
          (`KismetSystemLibrary.Delay` 0.2)
          (if (< _output_get _health)
            (`KismetSystemLibrary.PrintString` "Player already being healed" true true (struct :`R` 0.75 :`G` 0.412263 :`A` 1.0))
            (bind _returnvalue_2 (`self.K2_GetActorLocation` _asinssoldier))
            (set `self.Location` _returnvalue_2)
            (`self.Event_ShowLight_Yellow`)
            (`KismetSystemLibrary.Delay` 0.5 :!label _label)
            (`self.K2_DestroyActor`)
            (`KismetSystemLibrary.PrintString` "destroyed" true true (struct :`R` 1.0 :`B` 0.119809 :`A` 1.0))
            (else
              (set `self.Location` _returnvalue_2)
              (`self.Event_ShowLight_Green`)
              (set `self.SelfDestroySafety` true)
              (bind _asbp_od_med (cast `/OldDogs/Items/Utility/Meds/BP_OD_Med` (`self.GetOwner`)))
              (set `/OldDogs/Items/Utility/Meds/BP_OD_Med.MedsUsesCount` (+ (`/OldDogs/Items/Utility/Meds/BP_OD_Med.MedsUsesCount` _asbp_od_med) 1) _asbp_od_med)
              (`KismetSystemLibrary.PrintString` "Healing..." true true (struct :`R` 0.049854 :`G` 1.0 :`B` 0.17456 :`A` 1.0))
              (`/Engine/EditorBlueprintResources/StandardMacros.Gate` false :!label _label_2
                (:`Exit`
                  (if (`INSCharacter.bIsDying` _asinssoldier)
                    (`KismetSystemLibrary.PrintString` "Actor dead" true true (struct :`R` 0.713542 :`G` 0.65067 :`A` 1.0))
                    (elif _returnvalue
                      (set `INSCharacter.Health` (+ _health 0.25) _asinssoldier)
                      (`KismetSystemLibrary.Delay` 0.1)
                      (goto _label_2)
                      (else
                        (`KismetSystemLibrary.PrintString` "Healing done" true true (struct :`R` 0.658188 :`G` 0.150553 :`B` 0.78125 :`A` 1.0)))))
                  (`self.K2_DestroyActor`)))))
          (else
            (`KismetSystemLibrary.PrintString` "Player above 85% HP" true true (struct :`R` 0.75 :`G` 0.412263 :`A` 1.0))
            (set `self.Location` _returnvalue_2)
            (`self.Event_ShowLight_Red`)
            (goto _label))))
      (:`CastFailed`
        (`KismetSystemLibrary.PrintString` "Not soldier")
        (goto _label)))
    (else
      (`self.K2_DestroyActor`))))

(event `Event_ShowLight_Yellow`
  (if (not (`KismetSystemLibrary.IsServer`))
    (`KismetSystemLibrary.Delay` 0.2)
    (`GameplayStatics.SpawnEmitterAtLocation` "/OldDogs/Items/Utility/Meds/PS_OD_Meds_Working_Yellow.PS_OD_Meds_Working_Yellow" (`self.Location`) (struct) (5.0 5.0 5.0))
    (bind _asinsplayer_controller (cast `INSPlayerController` (`self.Info Message Target Proj`)))
    (`INSBasePlayerController.ClientMessageText` _asinsplayer_controller "Player already being healed" "None" 6.0)))

(event `Event_ShowLight_Red`
  (if (not (`KismetSystemLibrary.IsServer`))
    (`KismetSystemLibrary.Delay` 0.2)
    (`GameplayStatics.SpawnEmitterAtLocation` "/OldDogs/Items/Utility/Meds/PS_OD_Meds_Working_Red.PS_OD_Meds_Working_Red" (`self.Location`) (struct) (5.0 5.0 5.0))
    (bind _asinsplayer_controller (cast `INSPlayerController` (`self.Info Message Target Proj`)))
    (`INSBasePlayerController.ClientMessageText` _asinsplayer_controller "Player above 85% HP, can't be healed" "None" 6.0)))

(event `Event_ShowLight_Green`
  (bind _location (`self.Location`))
  (if (not (`KismetSystemLibrary.IsServer`))
    (`KismetSystemLibrary.Delay` 0.2)
    (`GameplayStatics.SpawnEmitterAtLocation` "/OldDogs/Items/Utility/Meds/PS_OD_Meds_Working_Green.PS_OD_Meds_Working_Green" _location (struct) (5.0 5.0 5.0))
    (`AkGameplayStatics.SpawnAkComponentAtLocation` "/Game/Audio/wwise/Sandstorm/VO/SecArabMale1/GeneralChatter2/Play_SecArabMale1_GeneralChatter2_Strenuous_Physical_Exertion.Play_SecArabMale1_GeneralChatter2_Strenuous_Physical_Exertion" _location (struct) true)
    (bind _asinsplayer_controller (cast `INSPlayerController` (`self.Info Message Target Proj`)))
    (`INSBasePlayerController.ClientMessageText` _asinsplayer_controller "Healing..." "None" 6.0)))

(fn `UserConstructionScript`)