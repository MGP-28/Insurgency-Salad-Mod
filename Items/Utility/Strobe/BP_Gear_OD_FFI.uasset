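; BP_Gear_OD_FFI is a utility gear item, an FFI strobe that shows a blinking light on the wearer.
; Shortly after BeginPlay it attaches a persistent emitter to the pelvis bone of the owner's third-person mesh.
; A Gate-fed Delay loop then repeatedly spawns a flash emitter at the same spot and destroys it moments later.
; The Gate starts open and nothing closes it, so the strobe runs continuously.
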(event `self.ReceiveBeginPlay`
  (bind _returnvalue (`self.GetOwnerMesh3P`))
  (`parent.ReceiveBeginPlay`)
  (`KismetSystemLibrary.Delay` 0.2)
  (`GameplayStatics.SpawnEmitterAttached` "/OldDogs/Items/Utility/Strobe/PS_OD_FFI.PS_OD_FFI" _returnvalue "b_ch_pelvis" (35.0 3.0 0.0) (struct) (1.0 1.0 1.0) "KeepRelativeOffset" false)
  (`/Engine/EditorBlueprintResources/StandardMacros.Gate` false :!label _label
    (:`Exit`
      (bind _returnvalue_2 (`GameplayStatics.SpawnEmitterAttached` "/OldDogs/Items/Utility/Strobe/PS_OD_FFI_Flash.PS_OD_FFI_Flash" _returnvalue "b_ch_pelvis" (35.0 3.0 0.0) (struct) (1.0 1.0 1.0) "KeepRelativeOffset" false))
      (`KismetSystemLibrary.Delay` 0.15)
      (`ActorComponent.K2_DestroyComponent` _returnvalue_2)
      (`KismetSystemLibrary.Delay` 0.25)
      (goto _label))))

(fn `UserConstructionScript`
  (`parent.UserConstructionScript`))