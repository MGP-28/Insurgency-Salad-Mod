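; Supply crate for flare ammo, marked unused by its asset name, that shows its remaining uses as instanced ammo box meshes.
; When uses left updates, it rebuilds all instances from stored transforms at full count, as on round reset, or otherwise removes one.
; A gated Tick loop, apparently for debugging, destroys flare ammo actors in the world one at a time with a short delay and on-screen messages.
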(event `self.BlueprintOnUsesLeftUpdated`
  (bind _ammomeshes (`self.AmmoMeshes`))
  (bind _usesleft (`self.UsesLeft`))
  (if (== (`self.TimesAllowedToBeUsed`) _usesleft)
    ;[1 1 1] This resets the Ammo Box Meshes on Round Reset
    (`InstancedStaticMeshComponent.ClearInstances` _ammomeshes)
    (for _index (range (`self.TimesAllowedToBeUsed`))
      (`InstancedStaticMeshComponent.AddInstance` _ammomeshes (`|GetArrayItem` (`self.AmmoMeshesTransforms`) _index)))
    (else
      (`InstancedStaticMeshComponent.RemoveInstance` _ammomeshes _usesleft))))

(event `self.ReceiveTick`
  (params (DeltaSeconds :type "Float (single-precision)"))
  (`/Engine/EditorBlueprintResources/StandardMacros.Gate` false :!label _label
    (:`Exit`
      (bind _outactors (`GameplayStatics.GetAllActorsOfClass` "/OldDogs/Items/Utility/Flare/BP_Grenade_OD_Flare_Ammo.BP_Grenade_OD_Flare_Ammo_C"))
      (bind _output (`|GetArrayItem` _outactors))
      (if (== _output null)
        (`KismetSystemLibrary.PrintString` "Nothing to destroy" true true (struct :`R` 0.96875 :`G` 1.0 :`B` 0.9375 :`A` 1.0) 5.0)
        (else
          (`self.K2_DestroyActor` _output)
          (`KismetSystemLibrary.PrintString` "Flare destroyed" true true (struct :`R` 1.0 :`G` 0.252639 :`B` 0.062211 :`A` 1.0) 5.0)))
      (`KismetSystemLibrary.Delay` 0.2)
      (goto _label))))

(fn `UserConstructionScript`)