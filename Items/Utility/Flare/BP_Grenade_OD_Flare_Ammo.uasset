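; BP_Grenade_OD_Flare_Ammo is an ammo flare grenade item that removes itself when too many ammo drops are already out.
; Half a second after BeginPlay, it looks up OD_Flare_Pallet and BP_Projectile_OD_Flare_Ammo_1 actors in the world.
; If pallets and flare projectiles together reach two, it calls DropItem and destroys itself.
; Each branch prints an on-screen debug message.
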(event `self.ReceiveBeginPlay`
  (`KismetSystemLibrary.Delay` 0.5)
  (bind _outactors (`GameplayStatics.GetAllActorsOfClass` "/OldDogs/Items/Utility/Flare/OD_Flare_Pallet.OD_Flare_Pallet_C"))
  (if (== (`|GetArrayItem` _outactors) null)
    (`KismetSystemLibrary.PrintString` "No pallets" true true (struct :`G` 1.0 :`B` 0.178514 :`A` 1.0) 5.0)
    (bind _outactors_2 (`GameplayStatics.GetAllActorsOfClass` "/OldDogs/Items/Utility/Flare/BP_Projectile_OD_Flare_Ammo_1.BP_Projectile_OD_Flare_Ammo_1_C"))
    (if (== (`|GetArrayItem` _outactors_2 1) null)
      (`KismetSystemLibrary.PrintString` "No pallets, less than 2 flares" true true (struct :`G` 1.0 :`B` 0.178514 :`A` 1.0) 5.0)
      (else
        (`KismetSystemLibrary.PrintString` "2 flares, removing" true true (struct :`R` 1.0 :`A` 1.0) 5.0)
        (`self.DropItem` :!label _label)
        (`self.K2_DestroyActor`)))
    (else
      (`KismetSystemLibrary.PrintString` "1 Pallet" true true (struct :`R` 1.0 :`G` 0.719981 :`A` 1.0) 5.0)
      (if (== (`|GetArrayItem` _outactors 1) null)
        (`KismetSystemLibrary.PrintString` "Only 1 pallet" true true (struct :`G` 1.0 :`B` 0.178514 :`A` 1.0) 5.0)
        (bind _outactors_3 (`GameplayStatics.GetAllActorsOfClass` "/OldDogs/Items/Utility/Flare/BP_Projectile_OD_Flare_Ammo_1.BP_Projectile_OD_Flare_Ammo_1_C"))
        (if (== (`|GetArrayItem` _outactors_3) null)
          (`KismetSystemLibrary.PrintString` "1 pallet, 0 flares" true true (struct :`G` 1.0 :`B` 0.178514 :`A` 1.0) 5.0)
          (else
            (`KismetSystemLibrary.PrintString` "1 pallet + 1 flare, removing" true true (struct :`R` 1.0 :`A` 1.0) 5.0)
            (goto _label)))
        (else
          (`KismetSystemLibrary.PrintString` "2 pallets, removing" true true (struct :`R` 1.0 :`A` 1.0) 5.0)
          (goto _label))))))

(fn `UserConstructionScript`)