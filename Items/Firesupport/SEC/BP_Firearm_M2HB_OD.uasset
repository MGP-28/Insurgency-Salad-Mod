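; M2HB heavy machine gun firearm that shows ammo-usage warning lights on its third-person mesh, apparently for a truck mount.
; Each fire event adds half a unit to a spent-ammo counter and prints it for debugging.
; A Gate and Delay loop started at BeginPlay polls that counter, attaching a yellow light emitter at the first threshold.
; At the second, it attaches a red one, destroys the yellow and stops polling.
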(event `self.ReceiveBeginPlay`
  (bind _returnvalue (`self.GetMesh3P`))
  (bind _fammospentx2 (`self.fAmmoSpentx2`))
  (`parent.ReceiveBeginPlay`)
  (`/Engine/EditorBlueprintResources/StandardMacros.Gate` false :!label _label
    (:`Exit`
      (if (>= _fammospentx2 250.0)
        (if (>= _fammospentx2 300.0)
          (`GameplayStatics.SpawnEmitterAttached` "/OldDogs/Items/Firesupport/Resources/PS_OD_TruckGunLight_Red.PS_OD_TruckGunLight_Red" _returnvalue "b_mntgn_mag_a09" (0.0 0.0 0.0) (struct) (1.0 1.0 1.0) "KeepRelativeOffset" false)
          (`ActorComponent.K2_DestroyComponent` (stale _returnvalue_2))
          (else
            (if (not (`self.bIsLightOn`))
              (bind _returnvalue_2 (`GameplayStatics.SpawnEmitterAttached` "/OldDogs/Items/Firesupport/Resources/PS_OD_TruckGunLight_Yellow.PS_OD_TruckGunLight_Yellow" _returnvalue "b_mntgn_mag_a09" (0.0 0.0 0.0) (struct) (1.0 1.0 1.0) "KeepRelativeOffset" false))
              (set `self.bIsLightOn` true))
            (`KismetSystemLibrary.Delay` 0.3 :!label _label_2)
            (goto _label)))
        (else
          (goto _label_2))))))

(event `self.BlueprintOnFire`
  (params (Origin :type "Vector Structure") (Direction :type "Vector Structure"))
  (bind _output_get (set `self.fAmmoSpentx2` (+ (`self.fAmmoSpentx2`) 0.5)))
  (`KismetSystemLibrary.PrintString` (`KismetStringLibrary.Conv_DoubleToString` _output_get)))

(fn `UserConstructionScript`
  (`parent.UserConstructionScript`))