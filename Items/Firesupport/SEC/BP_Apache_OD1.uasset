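; BP_Apache_OD1 is an Apache fire support helicopter with mounted weapons, destructible parts and a driver and gunner crew.
; On begin play it mounts an automatic M230 chaingun on the gunner's turret, wiring seat camera and aiming, plus two rocket pods.
; Destroyed rotors or engine, or a dying driver, start a fall.
; A badly damaged engine or dying gunner flags the AI blackboard to leave, with smoke and blood visuals marking damage.
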(event `self.ReceiveBeginPlay`
  (bind _gunnerseat (`self.GunnerSeat`))
  (`|ExecutionSequence`
    (:`then_0`
      ;[1 1 1] Attach Chaingun to Seat
      (`VehicleSeatComponent.SetCharacterAttachmentMesh` (`self.GunnerSeat`) (`self.VisibleMeshComponent`))
      (bind _returnvalue (`WeaponStatics.SpawnMountedWeapon` "/Game/Game/Actors/Weapons/HeavyMachineGun/BP_Firearm_M230.BP_Firearm_M230_C" self (`self.TurretYaw_L`) "pitch" (`self.GunnerSeat`)))
      (`/Engine/EditorBlueprintResources/StandardMacros.IsValid` _returnvalue
        (:`Is Valid`
          (`ItemFirearm.SetFiremode` _returnvalue "Automatic")
          (set `VehicleSeatComponent.CameraOffset` (.location (`SceneComponent.GetSocketTransform` (`ItemBase.GetMesh3P` _returnvalue) "camera" "RTS_Component")) _gunnerseat)
          (`VehicleSeatComponent.SetTurretComponents` _gunnerseat (`Actor.RootComponent` _returnvalue) (`self.TurretYaw_L`)))))
    (:`then_1`
      (`WeaponStatics.SpawnMountedWeapon` "/Game/Game/Actors/Weapons/Explosive/BP_Explosive_ApacheRockets.BP_Explosive_ApacheRockets_C" self (`self.RocketPodRight`) "None" null)
      (`WeaponStatics.SpawnMountedWeapon` "/Game/Game/Actors/Weapons/Explosive/BP_Explosive_ApacheRockets.BP_Explosive_ApacheRockets_C" self (`self.RocketPodLeft`) "None" null))))

(event `self.TailRotor.Delegate_OnPartDestroyed`
  (`ActorComponent.Activate` (`self.TailRotorSmoke`) false)
  (`self.StartFalling` true))

(event `self.EnginePart.Delegate_OnPartDestroyed`
  (`self.StartFalling` false))

(event `self.EnginePart.Delegate_OnPartDamaged`
  (params (VehiclePart :type "VehiclePartComponent Object Reference") (Damage :type "Float (single-precision)"))
  (if (< (`VehiclePartComponent.Health` VehiclePart) (* (`VehiclePartComponent.MaxHealth` VehiclePart) 0.25))
    (`/Engine/EditorBlueprintResources/StandardMacros.DoOnce` false
      (:`Completed`
        (`ActorComponent.Activate` (`self.EngineSmoke`) false)
        (`BlackboardComponent.SetValueAsBool` (`AIBlueprintHelperLibrary.GetBlackboard` self) "bShouldLeave" true)))))

(event `self.TopRotor.Delegate_OnPartDestroyed`
  (`self.StartFalling` false)
  (`ActorComponent.Activate` (`self.TopRotorSmoke`) false))

(event `self.DriverSeat.Delegate_OnSeatExited`
  (params (Character :type "INSCharacter Object Reference") (Seat :type "VehicleSeatComponent Object Reference"))
  (if (`INSCharacter.bIsDying` Character)
    (`SceneComponent.SetHiddenInGame` (`self.DriverBloodPlane3`) false false)
    (`SceneComponent.SetHiddenInGame` (`self.DriverBloodPlane2`) false false)
    (`SceneComponent.SetHiddenInGame` (`self.DriverBloodPlane1`) false false)
    (`self.StartFalling` false)))

(event `self.GunnerSeat.Delegate_OnSeatExited`
  (params (Character :type "INSCharacter Object Reference") (Seat :type "VehicleSeatComponent Object Reference"))
  (if (`INSCharacter.bIsDying` Character)
    (`SceneComponent.SetHiddenInGame` (`self.GunnerBloodPlane2`) false false)
    (`SceneComponent.SetHiddenInGame` (`self.GunnerBloodPlane3`) false false)
    (`SceneComponent.SetHiddenInGame` (`self.GunnerBloodPlane1`) false false)
    (`BlackboardComponent.SetValueAsBool` (`AIBlueprintHelperLibrary.GetBlackboard` self) "bShouldLeave" true)))

(fn `UserConstructionScript`)