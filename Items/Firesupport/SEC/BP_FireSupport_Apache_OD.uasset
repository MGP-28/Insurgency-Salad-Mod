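; Apache gunship fire support Blueprint for the Security faction that adds radio callouts when its weapons fire.
; OnWeaponFired checks the weapon class and has the INSGameMode broadcast a subtitled team radio event for rockets or the M230 chaingun.
; Separate flags limit each callout to the first firing of that weapon.
; Only the rocket broadcast passes the gunship's team ID explicitly.
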(event `self.OnWeaponFired`
  (params (HoveringVehicle :type "VehicleHoveringBase Object Reference") (Weapon :type "ItemFirearm Object Reference"))
  (bind _returnvalue (`GameplayStatics.GetObjectClass` Weapon))
  (bind _asinsgame_mode (cast `INSGameMode` (`GameplayStatics.GetGameMode`)))
  (`|ExecutionSequence`
    (:`then_0`
      (if (== _returnvalue "/Game/Game/Actors/Weapons/Explosive/BP_Explosive_ApacheRockets.BP_Explosive_ApacheRockets_C")
        (if (not (`self.bHasPlayedRockets`))
          (`INSGameMode.BroadcastTeamRadioEvent` _asinsgame_mode "/Game/Audio/wwise/Sandstorm/VO/Gunship/Play_Sec_Gunship_FiringRockets.Play_Sec_Gunship_FiringRockets" (`self.GetTeamId`) (`self.GetSubtitleText` "GunshipFiringRockets") self false 0.0 false false 10.0)
          (set `self.bHasPlayedRockets` true))))
    (:`then_1`
      (if (== _returnvalue "/Game/Game/Actors/Weapons/HeavyMachineGun/BP_Firearm_M230.BP_Firearm_M230_C")
        (if (not (`self.bHasPlayedChaingun`))
          (`INSGameMode.BroadcastTeamRadioEvent` _asinsgame_mode "/Game/Audio/wwise/Sandstorm/VO/Gunship/Play_Sec_Gunship_Attacking.Play_Sec_Gunship_Attacking" 0 (`self.GetSubtitleText` "SupportHelicopterGunshipEngaging") self false 0.0 false false 10.0)
          (set `self.bHasPlayedChaingun` true))))))

(fn `UserConstructionScript`)