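; Blackhawk fire-support helicopter (OD) with two gunner seats and AI that can be driven to leave or crash by damage.
; On BeginPlay it spawns an automatic GAU-19 on each turret yaw component and links it to its seat's camera and turret aiming.
; Destroying either rotor or the engine, or killing the pilot, starts a fall with matching smoke or blood effects.
; Low engine health triggers smoke and sets the blackboard's bShouldLeave flag.
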(event `self.ReceiveBeginPlay`
  (bind _turretyaw_l (`self.TurretYaw_L`))
  (bind _leftgunnerseat (`self.LeftGunnerSeat`))
  (bind _turretyaw_r (`self.TurretYaw_R`))
  (bind _rightgunnerseat (`self.RightGunnerSeat`))
  (`|ExecutionSequence`
    (:`then_0`
      ;[1 1 1] Attach Weapon Left
      (`VehicleSeatComponent.SetCharacterAttachmentMesh` (`self.LeftGunnerSeat`) (`self.VisibleMeshComponent`))
      (bind _returnvalue (`WeaponStatics.SpawnMountedWeapon` "/OldDogs/Items/Firesupport/SEC/BP_Firearm_GAU19_OD.BP_Firearm_GAU19_OD_C" self _turretyaw_l "pitch" _leftgunnerseat))
      (`/Engine/EditorBlueprintResources/StandardMacros.IsValid` _returnvalue
        (:`Is Valid`
          (`ItemFirearm.SetFiremode` _returnvalue "Automatic")
          (set `VehicleSeatComponent.CameraOffset` (.location (`SceneComponent.GetSocketTransform` (`ItemBase.GetMesh3P` _returnvalue) "camera" "RTS_Component")) (`self.LeftGunnerSeat`))
          (`VehicleSeatComponent.SetTurretComponents` _leftgunnerseat (`Actor.RootComponent` _returnvalue) _turretyaw_l))))
    (:`then_1`
      ;[1 1 1] Attach Weapon Right
      (`VehicleSeatComponent.SetCharacterAttachmentMesh` (`self.RightGunnerSeat`) (`self.VisibleMeshComponent`))
      (bind _returnvalue_2 (`WeaponStatics.SpawnMountedWeapon` "/OldDogs/Items/Firesupport/SEC/BP_Firearm_GAU19_OD.BP_Firearm_GAU19_OD_C" self _turretyaw_r "pitch" (`self.RightGunnerSeat`)))
      (`/Engine/EditorBlueprintResources/StandardMacros.IsValid` _returnvalue_2
        (:`Is Valid`
          (`ItemFirearm.SetFiremode` _returnvalue_2 "Automatic")
          (set `VehicleSeatComponent.CameraOffset` (.location (`SceneComponent.GetSocketTransform` (`ItemBase.GetMesh3P` _returnvalue_2) "camera" "RTS_Component")) _rightgunnerseat)
          (`VehicleSeatComponent.SetTurretComponents` _rightgunnerseat (`Actor.RootComponent` _returnvalue_2) _turretyaw_r))))))

(event `self.ReceiveTick`
  (params (DeltaSeconds :type "Float (single-precision)"))
  (set `self.Time` DeltaSeconds))

(event `self.TailRotor.Delegate_OnPartDestroyed`
  (`ActorComponent.Activate` (`self.TailRotorSmoke`) false)
  (`self.StartFalling` true))

(event `self.EnginePart.Delegate_OnPartDestroyed`
  (`self.StartFalling` false))

(event `self.TopRotor.Delegate_OnPartDestroyed`
  (`self.StartFalling` false)
  (`ActorComponent.Activate` (`self.TopRotorSmoke`) false))

(event `self.EnginePart.Delegate_OnPartDamaged`
  (params (VehiclePart :type "VehiclePartComponent Object Reference") (Damage :type "Float (single-precision)"))
  (if (< (`VehiclePartComponent.Health` VehiclePart) (* (`VehiclePartComponent.MaxHealth` VehiclePart) 0.25))
    (`/Engine/EditorBlueprintResources/StandardMacros.DoOnce` false
      (:`Completed`
        (`ActorComponent.Activate` (`self.EngineSmoke`) false)
        (`BlackboardComponent.SetValueAsBool` (`AIBlueprintHelperLibrary.GetBlackboard` self) "bShouldLeave" true)))))

(event `self.DriverSeat.Delegate_OnSeatExited`
  (params (Character :type "INSCharacter Object Reference") (Seat :type "VehicleSeatComponent Object Reference"))
  (if (`INSCharacter.bIsDying` Character)
    (`SceneComponent.SetHiddenInGame` (`self.DriverBloodPlane`) false false)
    (`self.StartFalling` false)))

(fn `UserConstructionScript`)