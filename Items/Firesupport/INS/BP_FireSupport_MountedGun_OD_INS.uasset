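; Insurgent fire support actor that delivers a shielded DShK mounted gun to the called-in target location.
; After a 12-second delay on BeginPlay it reads the artillery target location, and the server spawns the weapon there, ignoring collisions.
; The server then calls the SFX event, which plays a dust billow and supply-crate impact sound at that spot.
; Debug strings print on both the server and non-server branches.
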(event `self.ReceiveBeginPlay`
  (`KismetSystemLibrary.Delay` 12.0)
  (bind _returnvalue (`self.GetArtilleryTargetLocation`))
  (if (`KismetSystemLibrary.IsServer`)
    (`|SpawnActorFromClass` "/OldDogs/Items/Firesupport/INS/BP_MountedWeapon_DShK_Shield_OD.BP_MountedWeapon_DShK_Shield_OD_C" (`KismetMathLibrary.Conv_VectorToTransform` _returnvalue) "AlwaysSpawn" "OverrideRootScale" null null)
    (`self.SFX`)
    (else
      (`KismetSystemLibrary.PrintString` "Nono" true false (struct :`R` 1.0 :`A` 1.0) 15.0))))

(event `SFX`
  (`GameplayStatics.SpawnEmitterAtLocation` "/Game/Game/FX/Env/Dust/PS_DustBillow.PS_DustBillow" (stale `self.ReceiveBeginPlay` _returnvalue))
  (`AkGameplayStatics.SpawnAkComponentAtLocation` "/Game/Audio/wwise/Sandstorm/Vehicles/Air/C130/Play_C130_SupplyDrop_Crate_Impact.Play_C130_SupplyDrop_Crate_Impact" (stale `self.ReceiveBeginPlay` _returnvalue) (struct) true)
  (`KismetSystemLibrary.PrintString` "Boom" true false (struct :`R` 0.170582 :`G` 1.0 :`B` 0.839754 :`A` 1.0) 15.0))

(fn `UserConstructionScript`)