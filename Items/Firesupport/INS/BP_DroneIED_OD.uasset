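; BP_DroneIED_OD is an Insurgent (INS) fire-support IED quadcopter drone with damage and wreck behaviour.
; Part damage starts damage particles, while part destruction swaps in the wrecked material and animation, stops engine smoke and makes it fall.
; Further damage accumulates on the wreck until a threshold destroys the actor with dust and sound.
; A throttled, server-only stuck check on Tick counts low-movement samples, but takes no action.
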(event `self.ReceiveTick`
  (params (DeltaSeconds :type "Float (single-precision)"))
  (`self.CheckStuck`))

(event `self.VehicleDestructablePart.Delegate_OnPartDestroyed`
  (`ActorComponent.Activate` (`self.EngineSmoke`) false)
  (`PrimitiveComponent.SetMaterial` (`self.VisibleMeshComponent`) 0 "/Game/Animated/Vehicles/Driveable/Drone/MI_VH_INS_QuadCopter_Destroyed.MI_VH_INS_QuadCopter_Destroyed")
  (`self.StartFalling` true)
  (`SkeletalMeshComponent.SetAnimation` (`self.VisibleMeshComponent`) "/Game/Animated/Vehicles/Driveable/Drone/AN_VH_QuadCopter_Destroyed.AN_VH_QuadCopter_Destroyed")
  (set `self.bIsDestroyed` true))

(event `self.VehicleDestructablePart.Delegate_OnPartDamaged`
  (params (VehiclePart :type "VehiclePartComponent Object Reference") (Damage :type "Float (single-precision)"))
  (if (> (`VehiclePartComponent.Health` VehiclePart) 0.0)
    (`ActorComponent.Activate` (`self.DamageParticle`) true)))

(event `self.ReceiveAnyDamage`
  (params (Damage :type "Float (single-precision)") (DamageType :type "DamageType Object Reference") (InstigatedBy :type "Controller Object Reference") (DamageCauser :type "Actor Object Reference"))
  (bind _returnvalue (`self.K2_GetActorLocation`))
  (if (`self.bIsDestroyed`)
    (bind _output_get (set `self.DamageTakenWhileBroken` (+ (`self.DamageTakenWhileBroken`) Damage)))
    (if (>= _output_get 400.0)
      (`GameplayStatics.SpawnEmitterAtLocation` "/Game/Game/FX/Weapons/Generic/PS_DustKickup_Large.PS_DustKickup_Large" _returnvalue)
      (`AkGameplayStatics.SpawnAkComponentAtLocation` "/Game/Audio/wwise/Sandstorm/Physics/Dynamic_Props/Breakable/Play_Metal_Small_Breakable_Prop.Play_Metal_Small_Breakable_Prop" _returnvalue (struct) true)
      (`self.K2_DestroyActor`)
      (else
        (`KismetSystemLibrary.PrintString` "Broken but not destroyed" true true (struct :`R` 1.0 :`G` 1.0 :`A` 1.0))))
    (else
      (`KismetSystemLibrary.PrintString` "Not broken" true true (struct :`G` 1.0 :`A` 1.0)))))

(fn `CheckStuck`
  (bind _returnvalue (`self.K2_GetActorLocation`))
  (`/Engine/EditorBlueprintResources/ActorMacros.Switch Has Authority`
    (:`Authority`
      (if (`|EnumEquality` (`self.GetDamageState`) "DamageState_Alive")
        (if (not (> (+ (`self.LastStuckTest`) 1.0) (`GameplayStatics.GetTimeSeconds`)))
          (`|ExecutionSequence`
            (:`then_0`
              (set `self.LastStuckTest` (`GameplayStatics.GetTimeSeconds`)))
            (:`then_1`
              (`|ExecutionSequence`
                (:`then_0`
                  (if (< (`KismetMathLibrary.VSize` (- (`self.LastSampledLocation`) _returnvalue)) (`self.StuckThreshold`))
                    (`/Engine/EditorBlueprintResources/StandardMacros.IncrementInt` (`self.NumTimesStuck`)
                      (:`  `
                        (if (and (> (`self.NumTimesStuck`) 7) (`|EnumEquality` (`self.GetDamageState`) "DamageState_Alive"))
                          _)))
                    (else
                      (set `self.NumTimesStuck` 0))))
                (:`then_1`
                  (set `self.LastSampledLocation` _returnvalue))))))))))

(fn `UserConstructionScript`)