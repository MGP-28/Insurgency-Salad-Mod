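; Projectile Blueprint under the INS bot faction resources that pairs a vaporize-style burst effect with a follow-up OD Farto projectile.
; On BeginPlay, the server waits briefly, then spawns BP_Projectile_OD_Farto at the actor's current location, regardless of collision.
; The explode event plays the large character dismemberment Wwise sound and the vaporize dismemberment particle effect at the blast location.
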(event `self.ReceiveBeginPlay`
  (if (`KismetSystemLibrary.IsServer`)
    (`KismetSystemLibrary.Delay` 0.2)
    (`|SpawnActorFromClass` "/OldDogs/Items/Factions/Bots/INS/Resources/BP_Projectile_OD_Farto.BP_Projectile_OD_Farto_C" (`KismetMathLibrary.Conv_VectorToTransform` (`self.K2_GetActorLocation`)) "AlwaysSpawn" "OverrideRootScale" null null)))

(event `self.BlueprintOnExplode`
  (params (Location :type "Vector Structure (by ref)"))
  (`AkGameplayStatics.SpawnAkComponentAtLocation` "/Game/Audio/wwise/Sandstorm/Character/Dismemberment/Dismember/Play_Character_Dismemberment_Large.Play_Character_Dismemberment_Large" Location (struct) true)
  (`GameplayStatics.SpawnEmitterAtLocation` "/Game/Game/FX/Impacts/Flesh/PS_Impact_Dismember_Vaporize.PS_Impact_Dismember_Vaporize" Location))

(fn `UserConstructionScript`
  (`parent.UserConstructionScript`))