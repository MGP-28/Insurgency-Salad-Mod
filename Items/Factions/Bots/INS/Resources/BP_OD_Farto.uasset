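; BP_OD_Farto is an INS bot item that turns a swing into a suicide-bomber style detonation.
; On the server, BlueprintonSwing plays a metal detector alarm once, guarded by IsAlarmPlaying, then waits a short fuse delay.
; If the owning pawn is still alive, it spawns BP_Projectile_OD_Farto_Bang at its location and destroys its owner.
; The FartoEffects event holds dismemberment sound and vaporize particles, but nothing here calls it.
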(event `self.BlueprintOnSwing`
  (bind _returnvalue (`self.K2_GetActorLocation`))
  (if (`KismetSystemLibrary.IsServer`)
    (if (`self.bIsAlarmPlaying`)
      (`KismetSystemLibrary.PrintString` "Alarm already on")
      (else
        (set `self.bIsAlarmPlaying` true)
        (`AkGameplayStatics.SpawnAkComponentAtLocation` "/Game/Audio/wwise/Sandstorm/Physics/Dynamic_Props/Animated/MetalDetector/Play_metal_detector_alarm.Play_metal_detector_alarm" _returnvalue (struct) true)
        (`KismetSystemLibrary.Delay` 1.0)
        (if (> (`INSCharacter.Health` (`self.GetOwningPawn`)) 0.0)
          (`|SpawnActorFromClass` "/OldDogs/Items/Factions/Bots/INS/Resources/BP_Projectile_OD_Farto_Bang.BP_Projectile_OD_Farto_Bang_C" (`KismetMathLibrary.Conv_VectorToTransform` _returnvalue) "AlwaysSpawn" "OverrideRootScale" null null)
          (`self.K2_DestroyActor` (`self.GetOwner`))
          (else
            (`KismetSystemLibrary.PrintString` "Bot already dead")))))))

(event `Farto Effects`
  (bind _returnvalue (`self.K2_GetActorLocation`))
  (`AkGameplayStatics.SpawnAkComponentAtLocation` "/Game/Audio/wwise/Sandstorm/Character/Dismemberment/Dismember/Play_Character_Dismemberment_Large.Play_Character_Dismemberment_Large" _returnvalue (struct) true)
  (`GameplayStatics.SpawnEmitterAtLocation` "/Game/Game/FX/Impacts/Flesh/PS_Impact_Dismember_Vaporize.PS_Impact_Dismember_Vaporize" _returnvalue))

(fn `UserConstructionScript`
  (`parent.UserConstructionScript`))