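; Training weapon attachment that lets the siderail laser toggle point-shoot mode.
; From BeginPlay, a Gate and near-zero Delay loop polls the siderail WeaponLightComponent, flipping PSToggle each time its mode changes to Laser.
; Each flip makes the server message the instigating player controller that Point Shooting is enabled or disabled.
; ShouldEnterPointShootMode returns true only with a valid owning soldier, the toggle on and the laser active.
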(event `self.ReceiveBeginPlay`
  (`KismetSystemLibrary.Delay` 0.2)
  (set `self.Info Message Target` (`Actor.GetInstigatorController` (`self.GetOwner`)))
  (`/Engine/EditorBlueprintResources/StandardMacros.Gate` false :!label _label
    (:`Exit`
      (bind _asweapon_light_component (cast `WeaponLightComponent` (`ItemWeapon.GetUpgradeInSlot` (`self.OwningWeapon`) "Siderail")))
      (if (not (`self.bIsLightSwitchSet`))
        (bind _currentlightmode (`WeaponLightComponent.CurrentLightMode` _asweapon_light_component))
        (bind _output_get (set `self.LightSwitch` _currentlightmode))
        (set `self.bIsLightSwitchSet` true)
        (`KismetSystemLibrary.PrintString` (`|GetEnumeratorNameAsString` _output_get)))
      (if (not (`|EnumEquality` _currentlightmode (`self.LightSwitch`)))
        (set `self.LightSwitch` _currentlightmode)
        (if (`|EnumEquality` _currentlightmode "Laser")
          (if (`self.bPSToggle`)
            (set `self.bPSToggle` false)
            (`self.Laser Turned Off`)
            (else
              (set `self.bPSToggle` true)
              (`self.Laser Turned On`)))))
      (`KismetSystemLibrary.Delay` 0.0001)
      (goto _label))))

(event `Laser Turned On`
  (`KismetSystemLibrary.Delay` 0.2)
  (if (`KismetSystemLibrary.IsServer`)
    (bind _asinsplayer_controller (cast `INSPlayerController` (`self.Info Message Target`)))
    (`INSBasePlayerController.ClientMessageText` _asinsplayer_controller "Point Shooting ENABLED" "None" 2.5)))

(event `Laser Turned Off`
  (`KismetSystemLibrary.Delay` 0.2)
  (if (`KismetSystemLibrary.IsServer`)
    (bind _asinsplayer_controller (cast `INSPlayerController` (`self.Info Message Target`)))
    (`INSBasePlayerController.ClientMessageText` _asinsplayer_controller "Point Shooting DISABLED" "None" 2.5)))

(fn `ShouldEnterPointShootMode`
  (returns (ReturnValue :type Boolean))
  ;[0.0681 0.2448 0.04118] Enter point shoot mode if laser/flashlight activated
  (`/Engine/EditorBlueprintResources/StandardMacros.IsValid` (`self.GetOwningSoldier` self)
    (:`Is Valid`
      (bind _asweapon_light_component (cast `WeaponLightComponent` (`ItemWeapon.GetUpgradeInSlot` (`self.OwningWeapon`) "Siderail")))
      (if (`self.bPSToggle`)
        (if (`|EnumEquality` (`WeaponLightComponent.CurrentLightMode` _asweapon_light_component) "Laser")
          (return true)
          (else
            _))))
    (:`Is Not Valid`
      _))
  (return false))