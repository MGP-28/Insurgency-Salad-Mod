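; Deployed claymore projectile that uses a short-lived laser actor as its tripwire.
; After a five-second arming delay, the server repeatedly spawns and destroys OD_Claymore_Laser until one reports it has exploded.
; A melee slash from the instigator's controller spawns BP_Explosive_OD_Claymore just above it, with debug prints for each damage check.
; Destroying the claymore also destroys its current laser.
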(event `self.ReceiveBeginPlay`
  (if (`KismetSystemLibrary.IsServer`)
    (`KismetSystemLibrary.Delay` 5.0)
    (`/Engine/EditorBlueprintResources/StandardMacros.Gate` false :!label _label
      (:`Exit`
        (bind _returnvalue (`|SpawnActorFromClass` "/OldDogs/Items/Weapons/Explosives/Claymore/OD_Claymore_Laser.OD_Claymore_Laser_C" (`self.GetTransform`) "Undefined" "OverrideRootScale" self (`self.GetInstigator`)))
        (`KismetSystemLibrary.Delay` 0.005)
        (if (not (`/OldDogs/Items/Weapons/Explosives/Claymore/OD_Claymore_Laser.ExplodeOnceCheck` _returnvalue))
          (`self.K2_DestroyActor` _returnvalue)
          (goto _label))))))

(event `self.ReceiveDestroyed`
  (`self.K2_DestroyActor` (stale `self.ReceiveBeginPlay` _returnvalue)))

(event `self.ReceiveAnyDamage`
  (params (Damage :type "Float (single-precision)") (DamageType :type "DamageType Object Reference") (InstigatedBy :type "Controller Object Reference") (DamageCauser :type "Actor Object Reference"))
  (if (`KismetSystemLibrary.IsServer`)
    (if (== InstigatedBy (`self.GetInstigatorController`))
      (`KismetSystemLibrary.PrintString` "Owner" true true (struct :`G` 1.0 :`A` 1.0))
      (if (`KismetStringLibrary.EqualEqual_StrStr` (`KismetStringLibrary.Conv_ObjectToString` DamageType) "Default__DamageTypeMeleeSlash")
        (`KismetSystemLibrary.PrintString` "Knife" true true (struct :`G` 1.0 :`A` 1.0))
        (`|SpawnActorFromClass` "/OldDogs/Items/Weapons/Explosives/Claymore/BP_Explosive_OD_Claymore.BP_Explosive_OD_Claymore_C" (`KismetMathLibrary.MakeTransform` (+ (.location (`self.GetTransform`)) (* (`self.GetActorUpVector`) 30.0)) (.rotation (`self.GetTransform`)) (.scale (`self.GetTransform`))) "AdjustIfPossibleButAlwaysSpawn" "OverrideRootScale" null true null)
        (else
          (`KismetSystemLibrary.PrintString` "Not Knife" true true (struct :`R` 1.0 :`A` 1.0))))
      (else
        (`KismetSystemLibrary.PrintString` "Not owner" true true (struct :`R` 1.0 :`A` 1.0))))))

(fn `UserConstructionScript`)